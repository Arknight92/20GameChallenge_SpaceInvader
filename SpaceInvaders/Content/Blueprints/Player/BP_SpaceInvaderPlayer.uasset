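; Player spaceship pawn for a Space Invaders style game, with horizontal movement, shooting, score and respawn.
; Input sets a direction that Tick applies as a local offset, while tagged BP_BoundLimit overlaps block further movement toward that side.
; Only one projectile flies at a time; its destroy event re-enables shooting and awards enemy score to the game mode's UI widget.
; An explosion flipbook's finish triggers a delayed respawn, or destruction when no lives remain.
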(event OnComponentBeginOverlap(CapsuleCollision)
  (params (OverlappedComponent :type Primitive%20Component%20Object%20Reference) (OtherActor :type Actor%20Object%20Reference) (OtherComp :type Primitive%20Component%20Object%20Reference) (OtherBodyIndex :type Integer) (bFromSweep :type Boolean) (SweepResult :type Hit%20Result%20Structure%20%28by%20ref%29))
  (CallFunction|HandleBoundLimit OtherActor OtherActor OtherComp OtherComp))

(event OnFinishedPlaying(ExplosionAnimation)
  (Rendering|SetActorHiddenInGame true)
  (Utilities|FlowControl|Delay 0.5)
  (CallFunction|HandleRespawn))

(event Custom|EnableShoot
  (params (ActorCollided :type Actor%20Object%20Reference))
  (Variables|Default|SetCanShoot true)
  (CallFunction|CheckifEnnemyHit ActorCollided))

(event Input|EnhancedActionEvents|EnhancedInputActionIA_Shoot
  (params (ActionValue :type Boolean) (ElapsedSeconds :type Float%20%28double-precision%29) (TriggeredSeconds :type Float%20%28double-precision%29) (InputAction :type Input%20Action%20Object%20Reference :default "/Game/Blueprints/Inputs/InputActions/IA_Shoot.IA_Shoot"))
  (if (Variables|Default|GetCanShoot)
    (bind _projectile (CallFunction|SpawnProjectile))
    (Utilities|IsValid _projectile
      (:Is%20Valid
        (Default|SetShootOwner _projectile true)
        (EventDispatchers|BindEventtoOnProjectileDestroy _projectile (delegate Custom|EnableShoot))))))

(event Input|EnhancedActionEvents|EnhancedInputActionIA_MoveSpaceship
  (params (ActionValue :type Float%20%28double-precision%29) (ElapsedSeconds :type Float%20%28double-precision%29) (TriggeredSeconds :type Float%20%28double-precision%29) (InputAction :type Input%20Action%20Object%20Reference :default "/Game/Blueprints/Inputs/InputActions/IA_MoveSpaceship.IA_MoveSpaceship"))
  (:Started
    (bind _output_get (Variables|Default|SetDirectionValue ActionValue))
    ;[0.15 0.15 0.15 0.5] Prevent space ship to go through the hidden collision box
    (if (== _output_get (Variables|Default|GetCollidedBound))
      (Variables|Default|SetBlockMove true)
      (else
        (Variables|Default|SetCollidedBound 0.0)
        (Variables|Default|SetBlockMove false))))
  (:Completed
    (Variables|Default|SetDirectionValue 0.0)
    (Variables|Default|SetBlockMove false)))

(event EventBeginPlay
  (bind _asbp_space_invader_gm (Utilities|Casting|CastToBP_SpaceInvaderGM (Game|GetGameMode)))
  (Variables|Default|SetSpaceInvaderGM _asbp_space_invader_gm))

(event Collision|EventActorBeginOverlap
  (params (OtherActor :type Actor%20Object%20Reference)))

(event EventTick
  (params (DeltaSeconds :type Float%20%28single-precision%29))
  (CallFunction|HandleSpaceMovement DeltaSeconds))

(fn ConstructionScript)

(fn HandleSpaceMovement
  (params (DeltaSeconds :type Float%20%28double-precision%29))
  (if (not (Variables|Default|GetBlockMove))
    (Transformation|AddActorLocalOffset (Math|Vector|MakeVector (* (* (Variables|Default|GetSpaceshipSpeed) (Variables|Default|GetSpeedRate)) DeltaSeconds (Variables|Default|GetDirectionValue)) 0.0 0.0) false false)))

(fn SpawnProjectile
  (bind _returnvalue (Game|SpawnActorfromClass "/Game/Blueprints/Projectiles/BP_Projectile.BP_Projectile_C" (Math|Transform|MakeTransform (Transformation|GetWorldLocation (Variables|Default|GetShootSpawn)) "0, 0, 0" "1.000000,1.000000,1.000000") "AlwaysSpawn" "MultiplyWithRoot" 0 0))
  (Utilities|IsValid _returnvalue
    (:Is%20Valid
      (Variables|/Game/Blueprints/Projectiles/BP_Projectile.BP_Projectile_C|SetShootSpeed _returnvalue 1e+02)
      (Default|SetShootOwner _returnvalue true)
      (Variables|Default|SetCanShoot false)
      (return _returnvalue))))

(fn HandleBoundLimit
  (params (Object :type Object%20Object%20Reference) (Object2 :type Object%20Object%20Reference) (self2 :type Actor%20Component%20Object%20Reference) (self3 :type Actor%20Component%20Object%20Reference))
  (bind _returnvalue (Components|ComponentHasTag self2 "LeftLimit"))
  (bind _returnvalue_2 (Components|ComponentHasTag self3 "RightLimit"))
  (bind _directionvalue (Variables|Default|GetDirectionValue))
  (bind _directionvalue_2 (Variables|Default|GetDirectionValue))
  (bind _returnvalue_3 (> _directionvalue_2 0.0))
  (bind _returnvalue_4 (< _directionvalue 0.0))
  (bind _returnvalue_5 (and _returnvalue _returnvalue_4))
  (bind _returnvalue_6 (and _returnvalue_2 _returnvalue_3))
  (Development|PrintString (Utilities|GetDisplayName Object2))
  (if (== (Utilities|GetClass Object) "/Game/Blueprints/BP_BoundLimit.BP_BoundLimit_C")
    (if (or _returnvalue_6 _returnvalue_5)
      (Variables|Default|SetBlockMove true)
      (Development|PrintString "Block Move TRUE")
      (if _returnvalue_6
        (Variables|Default|SetCollidedBound 1.0)
        (elif _returnvalue_5
          (Variables|Default|SetCollidedBound -1.0))))))

(fn CheckifEnnemyHit
  (params (ActorHit :type Actor%20Object%20Reference))
  (bind _returnvalue (Utilities|GetClass ActorHit))
  (bind _spaceinvadergm (Variables|Default|GetSpaceInvaderGM))
  (bind _playeruiwidget (Variables|/Game/Blueprints/GameMode/BP_SpaceInvaderGM.BP_SpaceInvaderGM_C|GetPlayerUIWidget _spaceinvadergm))
  (bind _score_value (Variables|/Game/Blueprints/UI/BP_SpaceInvaderUI.BP_SpaceInvaderUI_C|GetScore_Value _playeruiwidget))
  (if (== _returnvalue "/Game/Blueprints/Ennemies/BP_Ennemy.BP_Ennemy_C")
    (bind _asbp_ennemy (Utilities|Casting|CastToBP_Ennemy ActorHit))
    (bind _output_get (Variables|Default|SetScore (+ (Variables|Default|GetScore) (Variables|/Game/Blueprints/Ennemies/BP_Ennemy.BP_Ennemy_C|GetScoreValue _asbp_ennemy))))
    (Rendering|Components|TextRender|SetText _score_value (Utilities|Text|ToText(String) (Utilities|String|ToString(Integer) _output_get)))
    (Default|LaunchExplosion _asbp_ennemy)
    (elif (== _returnvalue "/Game/Blueprints/Ennemies/BP_SpecialEnnemy.BP_SpecialEnnemy_C")
      (bind _asbp_special_ennemy (Utilities|Casting|CastToBP_SpecialEnnemy ActorHit))
      (bind _output_get_2 (Variables|Default|SetScore (+ (Variables|/Game/Blueprints/Ennemies/BP_Ennemy.BP_Ennemy_C|GetScoreValue _asbp_special_ennemy) (Variables|Default|GetScore))))
      (Rendering|Components|TextRender|SetText _score_value (Utilities|Text|ToText(Integer) _output_get_2))
      (Default|LaunchExplosion _asbp_special_ennemy))))

(fn LaunchExplosion
  (bind _explosionanimation (Variables|Default|GetExplosionAnimation))
  (Rendering|Components|Sprite|SetSprite (Variables|Default|GetPlayerSprite) 0)
  (Sprite|SetFlipbook _explosionanimation "/Game/Assets/SplitSprites/FB_OnHitEffect.FB_OnHitEffect")
  (Components|Timeline|SetLooping _explosionanimation false)
  (Components|Timeline|PlayfromStart _explosionanimation))

(fn HandleRespawn
  (if (> (Variables|Default|GetLives) 0)
    (Transformation|SetActorLocation "0.000000,0.000000,-30.000000" false true)
    (Sprite|SetFlipbook (Variables|Default|GetExplosionAnimation))
    (Rendering|Components|Sprite|SetSprite (Variables|Default|GetPlayerSprite) "/Game/Blueprints/Player/PlayerSprite.PlayerSprite")
    (Rendering|SetActorHiddenInGame false)
    (else
      (Actor|DestroyActor))))