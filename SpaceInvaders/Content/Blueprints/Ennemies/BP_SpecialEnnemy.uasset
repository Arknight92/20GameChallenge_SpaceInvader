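; BP_SpecialEnnemy is a special enemy that travels along its local X axis at a speed scaled by MoveRate.
; Tick applies the frame-rate independent movement.
; When its CollisionSphere overlaps a BP_BoundLimit component tagged RightLimit, it stops, waits briefly, then destroys itself.
; It also destroys itself when ExplosionAnimation finishes, while LaunchExplosion and construction simply defer to the parent class.
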(event OnComponentBeginOverlap(CollisionSphere)
  (params (OverlappedComponent :type Primitive%20Component%20Object%20Reference) (OtherActor :type Actor%20Object%20Reference) (OtherComp :type Primitive%20Component%20Object%20Reference) (OtherBodyIndex :type Integer) (bFromSweep :type Boolean) (SweepResult :type Hit%20Result%20Structure%20%28by%20ref%29))
  (if (and (== (Utilities|GetClass OtherActor) "/Game/Blueprints/BP_BoundLimit.BP_BoundLimit_C") (Components|ComponentHasTag OtherComp "RightLimit"))
    (Variables|Default|SetMoveRate 0.0)
    (Utilities|FlowControl|Delay 1.0)
    (Actor|DestroyActor)))

(event OnFinishedPlaying(ExplosionAnimation)
  (Actor|DestroyActor))

(event EventBeginPlay)

(event Collision|EventActorBeginOverlap
  (params (OtherActor :type Actor%20Object%20Reference)))

(event EventTick
  (params (DeltaSeconds :type Float%20%28single-precision%29))
  (Transformation|AddActorLocalOffset (Math|Vector|MakeVector (* DeltaSeconds (Variables|Default|GetMoveRate) 3e+01) 0.0 0.0) false false))

(fn ConstructionScript
  (|CallParentFunction))

(fn LaunchExplosion
  (|CallParentFunction))