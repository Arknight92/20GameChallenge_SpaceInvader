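; Enemy actor for a Space Invaders game that steps sideways or down, fires projectiles and explodes on death.
; MoveEnnemy applies each step, while overlaps with BP_BoundLimit set the game mode's shared direction and descent flags, clearing descent after a downward step.
; LaunchExplosion plays a hit flipbook, whose completion reports the enemy and its grid indices to the game mode, then calls OnEnemyDeath.
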(event OnComponentBeginOverlap(CollisionSphere)
  (params (OverlappedComponent :type Primitive%20Component%20Object%20Reference) (OtherActor :type Actor%20Object%20Reference) (OtherComp :type Primitive%20Component%20Object%20Reference) (OtherBodyIndex :type Integer) (bFromSweep :type Boolean) (SweepResult :type Hit%20Result%20Structure%20%28by%20ref%29))
  (CallFunction|HandleBoundLimit OtherActor OtherComp))

(event OnFinishedPlaying(ExplosionAnimation)
  (bind _indexx (Variables|Default|GetIndexX))
  (bind _indexy (Variables|Default|GetIndexY))
  (Development|PrintString "EXPLOSION ENDED" true true "(R=1.000000,G=0.335289,B=0.000000,A=1.000000)")
  (bind _asbp_space_invader_gm (Utilities|Casting|CastToBP_SpaceInvaderGM (Game|GetGameMode)))
  (Utilities|Array|Add (Variables|/Game/Blueprints/GameMode/BP_SpaceInvaderGM.BP_SpaceInvaderGM_C|GetIndexToRemove _asbp_space_invader_gm) _indexx)
  (Utilities|Array|Add (Variables|/Game/Blueprints/GameMode/BP_SpaceInvaderGM.BP_SpaceInvaderGM_C|GetIndexToRemove _asbp_space_invader_gm) _indexy)
  (Development|PrintString (Utilities|String|Append "Index X = " (Utilities|String|ToString(Integer) _indexx)))
  (Development|PrintString (Utilities|String|Append "Index Y = " (Utilities|String|ToString(Integer) _indexy)))
  (Variables|/Game/Blueprints/GameMode/BP_SpaceInvaderGM.BP_SpaceInvaderGM_C|SetEnnemyDestroyed _asbp_space_invader_gm self)
  (Default|CallOnEnemyDeath))

(event Custom|MoveEnnemy
  (params (DoWeMoveRight :type Boolean) (DoWeMoveDown :type Boolean))
  (CallFunction|SetHorizontalMove DoWeMoveRight)
  (CallFunction|SetVerticalMove DoWeMoveDown))

(event EventBeginPlay
  (bind _asbp_space_invader_gm (Utilities|Casting|CastToBP_SpaceInvaderGM (Game|GetGameMode))))

(event Collision|EventActorBeginOverlap
  (params (OtherActor :type Actor%20Object%20Reference)))

(event EventTick
  (params (DeltaSeconds :type Float%20%28single-precision%29))
  (if (Variables|Default|GetIsExplosionLaunch)
    _))

(fn ConstructionScript)

(fn SetEnnemySprite
  (params (Sprite :type Paper%20Sprite%20Object%20Reference)))

(fn SetHorizontalMove
  (params (Condition :type Boolean))
  (if Condition
    (Variables|Default|SetDirectionX 1.0)
    (else
      (Variables|Default|SetDirectionX -1.0)))
  (Variables|Default|SetMoveY 0.0))

(fn HandleBoundLimit
  (params (Actor :type Actor%20Object%20Reference) (Component :type Actor%20Component%20Object%20Reference))
  (if (== (Utilities|GetClass Actor) "/Game/Blueprints/BP_BoundLimit.BP_BoundLimit_C")
    (bind _asbp_space_invader_gm (Utilities|Casting|CastToBP_SpaceInvaderGM (Game|GetGameMode)))
    (if (Components|ComponentHasTag Component "RightLimit")
      (Variables|/Game/Blueprints/GameMode/BP_SpaceInvaderGM.BP_SpaceInvaderGM_C|SetMoveRight _asbp_space_invader_gm false)
      (if (not (Variables|/Game/Blueprints/GameMode/BP_SpaceInvaderGM.BP_SpaceInvaderGM_C|GetMoveDown _asbp_space_invader_gm)) :!label _label
        (Variables|/Game/Blueprints/GameMode/BP_SpaceInvaderGM.BP_SpaceInvaderGM_C|SetMoveDown _asbp_space_invader_gm true)
        (Development|PrintString "MoveDown Changed" false))
      (elif (Components|ComponentHasTag Component "LeftLimit")
        (Variables|/Game/Blueprints/GameMode/BP_SpaceInvaderGM.BP_SpaceInvaderGM_C|SetMoveRight _asbp_space_invader_gm true)
        (goto _label)))))

(fn SpawnProjectile
  (Development|PrintString "Spawn Ennemy Projectile")
  (bind _returnvalue (Game|SpawnActorfromClass "/Game/Blueprints/Projectiles/BP_Projectile.BP_Projectile_C" (Math|Transform|MakeTransform (Transformation|GetWorldLocation (Variables|Default|GetShootSpawn)) "0, 0, 0" "1.000000,1.000000,1.000000") "AlwaysSpawn" "MultiplyWithRoot" 0 0))
  (Utilities|IsValid _returnvalue
    (:Is%20Valid
      (Default|SetShootOwner _returnvalue false)
      (return _returnvalue))))

(fn SetVerticalMove
  (params (Condition :type Boolean))
  (if Condition
    (Variables|Default|SetMoveY -2e+01)
    (Variables|Default|SetDirectionX 0.0)
    (Development|PrintString "Should Move Ennemy Down" true true "(R=1.000000,G=0.000000,B=0.057429,A=1.000000)"))
  (Transformation|AddActorLocalOffset (Math|Vector|MakeVector (* (Variables|Default|GetMoveX) (Variables|Default|GetDirectionX)) 0.0 (Variables|Default|GetMoveY)) false false)
  (if (< (Variables|Default|GetMoveY) 0.0)
    (bind _asbp_space_invader_gm (Utilities|Casting|CastToBP_SpaceInvaderGM (Game|GetGameMode)))
    (Variables|/Game/Blueprints/GameMode/BP_SpaceInvaderGM.BP_SpaceInvaderGM_C|SetMoveDown _asbp_space_invader_gm false)
    (Development|PrintString (Utilities|String|ToString(Boolean) (Variables|/Game/Blueprints/GameMode/BP_SpaceInvaderGM.BP_SpaceInvaderGM_C|GetMoveRight _asbp_space_invader_gm)) true true "(R=1.000000,G=0.756040,B=0.000000,A=1.000000)")))

(fn LaunchExplosion
  (bind _explosionanimation (Variables|Default|GetExplosionAnimation))
  (Rendering|Components|Sprite|SetSprite (Variables|Default|GetEnnemySprite) 0)
  (Sprite|SetFlipbook _explosionanimation "/Game/Assets/SplitSprites/FB_OnHitEffect.FB_OnHitEffect")
  (Components|Timeline|SetLooping _explosionanimation false)
  (Variables|Default|SetIsExplosionLaunch true))

(fn DestroyThisEnnemy
  (Actor|DestroyActor))