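; Paper2D projectile shared by the player and aliens, flying vertically as a beam shot.
; SetShootOwner tags the shooter as Player or Alien, picks the matching flipbook and travel direction, then arms movement.
; Once the owner is set, Tick offsets the actor along local Z by speed, rate multiplier, direction and delta time.
; The Blueprint itself contains no collision, damage or destruction logic.
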(event EventBeginPlay)

(event Collision|EventActorBeginOverlap
  (params (OtherActor :type Actor%20Object%20Reference)))

(event EventTick
  (params (DeltaSeconds :type Float%20%28single-precision%29))
  (if (Variables|Default|GetOwnerSet)
    (Transformation|AddActorLocalOffset (Math|Vector|MakeVector 0.0 0.0 (* (Variables|Default|GetShootSpeed) DeltaSeconds (Variables|Default|GetSpeedRate) (Variables|Default|GetShootDirection))) false false)))

(fn ConstructionScript)

(fn SetShootOwner
  (params (IsPlayer :type Boolean))
  (if IsPlayer
    (Variables|Default|SetShootOwner "Player")
    (Variables|Default|SetShootDirection 1.0)
    (Variables|Default|SetSelectedFlipbook "/Game/Assets/SplitSprites/FB_SpaceBeam_Flipbook.FB_SpaceBeam_Flipbook")
    (else
      (Variables|Default|SetShootOwner "Alien")
      (Variables|Default|SetShootDirection -1.0)
      (Variables|Default|SetSelectedFlipbook "/Game/Assets/SplitSprites/FB_EnnemyBeam.FB_EnnemyBeam")))
  (Sprite|SetFlipbook (Variables|Default|GetProjectileSprite) (Variables|Default|GetSelectedFlipbook))
  (Variables|Default|SetOwnerSet true))