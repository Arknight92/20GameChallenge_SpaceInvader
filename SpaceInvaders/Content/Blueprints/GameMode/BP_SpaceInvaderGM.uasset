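; Space Invaders game mode that spawns the enemy grid and UI, drives enemy movement and shooting, and tracks player lives.
; Looping timers broadcast grid movement and fire from a random shooter, initially drawn from the bottom row.
; Enemy death events remove the enemy from both arrays and can promote the one above it to shooter.
; Player hits trigger an explosion, cost a life and darken its icon; game over only prints a message.
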(event Custom|UpdateShootingArray
  (bind _ennemyarray (Variables|Default|GetEnnemyArray))
  (bind _shootingennemies (Variables|Default|GetShootingEnnemies))
  (Development|PrintString (Utilities|String|Append "In Call back update Shoot Array and ennemy to destroy has index " (Utilities|String|ToString(Integer) (Variables|/Game/Blueprints/Ennemies/BP_Ennemy.BP_Ennemy_C|GetIndexX (Variables|Default|GetEnnemyDestroyed))) ":" (Utilities|String|ToString(Integer) (Variables|/Game/Blueprints/Ennemies/BP_Ennemy.BP_Ennemy_C|GetIndexY (Variables|Default|GetEnnemyDestroyed)))) true true "(R=1.000000,G=0.013603,B=0.000000,A=1.000000)")
  (CallFunction|RemoveEnnemyfromArray _ennemyarray _ennemyarray (stale EventBeginPlay _array_element))
  (CallFunction|RemoveEnnemyfromArray _shootingennemies _shootingennemies (stale EventBeginPlay _array_element))
  (Development|PrintString (Utilities|String|Append "Shooting Ennemies size " (Utilities|String|ToString(Integer) (Utilities|Array|Length (Variables|Default|GetShootingEnnemies)))) true true "(R=1.000000,G=0.756040,B=0.000000,A=1.000000)")
  (CallFunction|SetNewShootingEnnemy)
  (Utilities|Array|Clear (Variables|Default|GetIndexToRemove))
  (Utilities|IsValid (Variables|Default|GetEnnemyDestroyed)
    (:Is%20Valid
      (Actor|DestroyActor (Variables|Default|GetEnnemyDestroyed))
      (Variables|Default|SetEnnemyDestroyed 0))))

(event Custom|OnPlayerOrBunkerHit
  (params (ActorCollided :type Actor%20Object%20Reference))
  (if (== (Utilities|GetClass ActorCollided) "/Game/Blueprints/Player/BP_SpaceInvaderPlayer.BP_SpaceInvaderPlayer_C")
    (bind _asbp_space_invader_player (Utilities|Casting|CastToBP_SpaceInvaderPlayer ActorCollided))
    (Default|LaunchExplosion _asbp_space_invader_player)
    (CallFunction|SetPlayerLivesUI (Variables|/Game/Blueprints/Player/BP_SpaceInvaderPlayer.BP_SpaceInvaderPlayer_C|GetLives _asbp_space_invader_player))
    (bind _output_get (Variables|/Game/Blueprints/Player/BP_SpaceInvaderPlayer.BP_SpaceInvaderPlayer_C|SetLives _asbp_space_invader_player (- (Variables|/Game/Blueprints/Player/BP_SpaceInvaderPlayer.BP_SpaceInvaderPlayer_C|GetLives _asbp_space_invader_player) 1)))
    (CallFunction|HandlePlayerRespawn _output_get)))

(event EventBeginPlay
  (bind _returnvalue (UserInterface|CreateWidget "/Game/Blueprints/UI/BP_SpaceInvaderUI.BP_SpaceInvaderUI_C"))
  (Variables|Default|SetPlayerUIWidget _returnvalue)
  (UserInterface|Viewport|AddtoViewport _returnvalue 0)
  (CallFunction|InitializeLivesArray)
  (CallFunction|SpawnEnnemiesGrid)
  (CallFunction|InitializeEnnemyShooting)
  (for _array_element (Variables|Default|GetEnnemyArray)
    (EventDispatchers|BindEventtoOnEnemyDeath _array_element (delegate Custom|UpdateShootingArray))
    (Development|PrintString (Utilities|String|ToString(Vector2d) (Viewport|GetViewportSize))))
  (Utilities|Time|SetTimerbyFunctionName 0 "CallMoveGridDispatcher" (Variables|Default|GetMoveRate) true)
  (Utilities|Time|SetTimerbyFunctionName 0 "SelectRandomShooter" (* (Variables|Default|GetMoveRate) 1.5) true))

(event EventTick
  (params (DeltaSeconds :type Float%20%28single-precision%29)))

(fn ConstructionScript)

(fn SpawnEnnemiesGrid
  (bind _firstenemylocation (Variables|Default|GetFirstEnemyLocation))
  (for _index (range 0 (- (Variables|Default|GetRowNumber) 1))
    (for _index_2 (range 0 (- (Variables|Default|GetColumnNumber) 1))
      (bind _returnvalue (Game|SpawnActorfromClass "/Game/Blueprints/Ennemies/BP_Ennemy.BP_Ennemy_C" (Math|Transform|MakeTransform (Math|Vector|MakeVector (+ (.x _firstenemylocation) (* _index_2 (Variables|Default|GetTranslationX))) 0.0 (- (.z _firstenemylocation) (* _index (Variables|Default|GetTranslationZ)))) "0, 0, 0" "1.000000,1.000000,1.000000") "AlwaysSpawn" "MultiplyWithRoot" 0 0))
      (Rendering|Components|Sprite|SetSprite (Variables|/Game/Blueprints/Ennemies/BP_Ennemy.BP_Ennemy_C|GetEnnemySprite _returnvalue) (Utilities|Array|Get(acopy) (Variables|Default|GetSpriteArray) _index))
      (Variables|/Game/Blueprints/Ennemies/BP_Ennemy.BP_Ennemy_C|SetIndexX _returnvalue _index)
      (Variables|/Game/Blueprints/Ennemies/BP_Ennemy.BP_Ennemy_C|SetIndexY _returnvalue _index_2)
      (Variables|/Game/Blueprints/Ennemies/BP_Ennemy.BP_Ennemy_C|SetScoreValue _returnvalue (* (- (Variables|Default|GetRowNumber) _index_2) 10))
      (Utilities|Array|Add (Variables|Default|GetEnnemyArray) _returnvalue)))
  (Variables|Default|SetEnableMove true))

(fn CallMoveGridDispatcher
  (Default|CallCallMoveGrid (Variables|Default|GetMoveRight) (Variables|Default|GetMoveDown)))

(fn InitializeEnnemyShooting
  (for _array_element (Variables|Default|GetEnnemyArray)
    (if (== (Variables|/Game/Blueprints/Ennemies/BP_Ennemy.BP_Ennemy_C|GetIndexX _array_element) (- (Variables|Default|GetRowNumber) 1))
      (Utilities|Array|Add (Variables|Default|GetShootingEnnemies) _array_element))))

(fn SelectRandomShooter
  (bind _shootingennemies (Variables|Default|GetShootingEnnemies))
  (if (Utilities|Array|IsNotEmpty _shootingennemies)
    (bind _projectile (Default|SpawnProjectile (.OutItem (Utilities|Array|Random _shootingennemies))))
    (Utilities|IsValid _projectile
      (:Is%20Valid
        (Default|SetShootOwner _projectile false)
        (EventDispatchers|BindEventtoOnProjectileDestroy _projectile (EventDispatchers|CreateEvent :!event Custom|OnPlayerOrBunkerHit))))))

(fn Dead
  (Development|PrintString "DEATH MOTHERFUCKER"))

(fn RemoveEnnemyfromArray
  (params (Array :type Array%20of%20BP%20Ennemy%20Object%20References) (TargetArray :type Array%20of%20BP%20Ennemy%20Object%20References) (Item :type BP%20Ennemy%20Object%20Reference%20%28by%20ref%29))
  (Development|PrintString (Utilities|String|Append "Before Loop, array size  = " (Utilities|String|ToString(Integer) (Utilities|Array|Length Array))) true true "(R=1.000000,G=0.000000,B=0.057429,A=1.000000)")
  (bind (_array_element _array_index) (Utilities|Array|ForEachLoopwithBreak Array :!label _label)
    (:LoopBody
      (if (and (== (Utilities|Array|Get(acopy) (Variables|Default|GetIndexToRemove)) (Variables|/Game/Blueprints/Ennemies/BP_Ennemy.BP_Ennemy_C|GetIndexX _array_element)) (== (Utilities|Array|Get(acopy) (Variables|Default|GetIndexToRemove) 1) (Variables|/Game/Blueprints/Ennemies/BP_Ennemy.BP_Ennemy_C|GetIndexY _array_element)))
        (Development|PrintString (Utilities|String|Append "Removed ennemy with indexes: " (Utilities|String|ToString(Integer) (Variables|/Game/Blueprints/Ennemies/BP_Ennemy.BP_Ennemy_C|GetIndexX _array_element)) ":" (Utilities|String|ToString(Integer) (Variables|/Game/Blueprints/Ennemies/BP_Ennemy.BP_Ennemy_C|GetIndexY _array_element))) true true "(R=1.000000,G=0.039894,B=0.000000,A=1.000000)")
        (Utilities|Array|RemoveIndex TargetArray _array_index)
        (goto _label Break)))
    (:Completed
      (Development|PrintString (Utilities|String|Append "exiting Remove Ennmy From array " (Utilities|String|ToString(Integer) (Utilities|Array|Length TargetArray))) true true "(R=1.000000,G=0.000000,B=0.140383,A=1.000000)"))))

(fn SetNewShootingEnnemy
  (bind _ennemyarray (Variables|Default|GetEnnemyArray))
  (bind _indextoremove (Variables|Default|GetIndexToRemove))
  (bind _shootingennemies (Variables|Default|GetShootingEnnemies))
  (bind _indextoremove_2 (Variables|Default|GetIndexToRemove))
  (bind _array_element (Utilities|Array|ForEachLoopwithBreak _ennemyarray :!label _label)
    (:LoopBody
      (if (and (> (Variables|/Game/Blueprints/Ennemies/BP_Ennemy.BP_Ennemy_C|GetIndexX _array_element) (Utilities|Array|Get(acopy) _indextoremove_2)) (== (Variables|/Game/Blueprints/Ennemies/BP_Ennemy.BP_Ennemy_C|GetIndexY _array_element) (Utilities|Array|Get(acopy) _indextoremove_2 1)))
        (LocalVariables|SetNeedToReplaceShooter false)
        (goto _label Break)))
    (:Completed
      (bind _array_element_2 (Utilities|Array|ForEachLoopwithBreak _ennemyarray :!label _label_2)
        (:LoopBody
          (if (Math|Boolean|ANDBoolean (== (- (Utilities|Array|Get(acopy) _indextoremove) 1) (Variables|/Game/Blueprints/Ennemies/BP_Ennemy.BP_Ennemy_C|GetIndexX _array_element_2)) (== (Utilities|Array|Get(acopy) _indextoremove 1) (Variables|/Game/Blueprints/Ennemies/BP_Ennemy.BP_Ennemy_C|GetIndexY _array_element_2)) (LocalVariables|GetNeedToReplaceShooter))
            (Development|PrintString (Utilities|String|Append "Index to add" (Utilities|String|ToString(Integer) (Utilities|Array|Get(acopy) (Variables|Default|GetIndexToRemove) 1))))
            (Utilities|Array|Add _shootingennemies _array_element_2)
            (goto _label_2 Break)))
        (:Completed
          (Development|PrintString (Utilities|String|Append "Array shooting new size: " (Utilities|String|ToString(Integer) (Utilities|Array|Length _shootingennemies))) true true "(R=1.000000,G=0.000000,B=0.057429,A=1.000000)"))))))

(fn AreAllEnnemiesDead
  (return (Utilities|Array|IsEmpty (Variables|Default|GetEnnemyArray))))

(fn InitializeLivesArray
  (bind _playeruiwidget (Variables|Default|GetPlayerUIWidget))
  (bind _livesarray (Variables|Default|GetLivesArray))
  (Utilities|Array|Add _livesarray (Variables|/Game/Blueprints/UI/BP_SpaceInvaderUI.BP_SpaceInvaderUI_C|GetLife_1 _playeruiwidget))
  (Utilities|Array|Add _livesarray (Variables|/Game/Blueprints/UI/BP_SpaceInvaderUI.BP_SpaceInvaderUI_C|GetLife_2 _playeruiwidget))
  (Utilities|Array|Add _livesarray (Variables|/Game/Blueprints/UI/BP_SpaceInvaderUI.BP_SpaceInvaderUI_C|GetLife_3 _playeruiwidget)))

(fn SetPlayerLivesUI
  (params (PlayerCurrentLife :type Integer))
  (Variables|/Script/UMG.Image|SetColorAndOpacity (Utilities|Array|Get(acopy) (Variables|Default|GetLivesArray) (- PlayerCurrentLife 1)) (Utilities|Struct|MakeLinearColor 0.0 0.0 0.0 1.0)))

(fn HandlePlayerRespawn
  (params (PlayerCurrentLives :type Integer))
  (if (<= PlayerCurrentLives 0)
    (Development|PrintString "GAME OVER !!")))